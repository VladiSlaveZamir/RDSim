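; BP_Track_Test is a test track actor that spawns ring actors along a spline and debugs whether its points sit on the ground.
; On BeginPlay it spawns a BP_Ring_Test at each spline point, matching location and rotation.
; Every Tick it draws a visibility trace from each point down to a fixed world height, then prints "Ground" for very close hits and "Air" otherwise.
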(event `self.ReceiveBeginPlay`
  (bind _spline (`self.Spline`))
  (for _index (range (+ (`SplineComponent.GetNumberOfSplinePoints` (`self.Spline`)) 1))
    (`|SpawnActorFromClass` "/Game/RDSim/Blueprint/Track/BP_Ring_Test.BP_Ring_Test_C" (`KismetMathLibrary.MakeTransform` (`SplineComponent.GetLocationAtSplinePoint` _spline _index "World") (`SplineComponent.GetRotationAtSplinePoint` _spline _index "World")) "AlwaysSpawn" "OverrideRootScale" null null)))

(event `self.ReceiveTick`
  (params (DeltaSeconds :type "Float (single-precision)"))
  (for _index (range (+ (`SplineComponent.GetNumberOfSplinePoints` (`self.Spline`)) 1))
    (bind _returnvalue (`SplineComponent.GetLocationAtSplinePoint` (`self.Spline`) _index "World"))
    (bind _outhit (`KismetSystemLibrary.LineTraceSingle` :`Start` _returnvalue :`End` (`KismetMathLibrary.MakeVector` (.x _returnvalue) (.y _returnvalue) -1.0) :`TraceChannel` "TraceTypeQuery1" :`DrawDebugType` "ForOneFrame"))
    (bind (_bblockinghit _binitialoverlap _time _distance) (`GameplayStatics.BreakHitResult` _outhit))
    (if _bblockinghit
      (if (> _distance 1.0)
        (`KismetSystemLibrary.PrintString` "Air" :!label _label)
        (else
          (`KismetSystemLibrary.PrintString` "Ground")))
      (else
        (goto _label)))))

(fn `UserConstructionScript`)