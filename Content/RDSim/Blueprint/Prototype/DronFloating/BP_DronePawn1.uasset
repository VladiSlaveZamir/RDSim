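; Prototype drone pawn flown with gamepad thumbsticks.
; The right stick drives timeline-eased horizontal movement along world X and Y, while the left stick yaws and lifts it.
; A downward line trace on Tick measures height so descent slows near the ground.
; Looping timers spin the four propellers in opposing pairs and smoothly tilt the body mesh toward the right stick input.
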(event `InputAxis|Right Thumbstrick X`
  (params (AxisValue :type "Float (single-precision)"))
  (bind _returnvalue (`GameplayStatics.GetWorldDeltaSeconds`))
  ;[1 1 1] XYMove
  (`|ExecutionSequence`
    (:`then_0`
      (if (> AxisValue 0.0)
        (bind (_direction _newtrack_0) (`Timeline|Timeline_1` :!label _label)
          (:`Update`
            (bind _output_get (set `self.Speed` _newtrack_0))
            (`self.AddMovementInput` (`KismetMathLibrary.MakeVector` 0.0 (`KismetMathLibrary.FInterpTo` 0.0 _output_get _returnvalue 1.0)))))
        (else
          (goto _label :!via `Reverse`))))
    (:`then_1`
      (if (< AxisValue 0.0)
        (bind (_direction_2 _newtrack_0_2) (`Timeline|Timeline_2` :!label _label_2)
          (:`Update`
            (bind _output_get_2 (set `self.Speed` _newtrack_0_2))
            (`self.AddMovementInput` (`KismetMathLibrary.MakeVector` 0.0 (`KismetMathLibrary.FInterpTo` 0.0 _output_get_2 _returnvalue 1.0)))))
        (else
          (goto _label_2 :!via `Reverse`))))))

(event `self.ReceiveBeginPlay`
  ;[1 1 1] Propeller and Body Rotation
  (`KismetSystemLibrary.K2_SetTimerDelegate` (`|CreateDelegate` :!event `Propeller Rotation Tick`) 0.01 true)
  (`KismetSystemLibrary.K2_SetTimerDelegate` (`|CreateDelegate` :!event `Body RotationTick`) 0.01 true))

(event `Propeller Rotation Tick`
  ;[1 1 1] Rotation propellers
  (`SceneComponent.K2_AddRelativeRotation` (`self.Propeller2`) (struct :`Yaw` 3500.0) false false)
  (`SceneComponent.K2_AddRelativeRotation` (`self.Propeller4`) (struct :`Yaw` 3500.0) false false)
  (`SceneComponent.K2_AddRelativeRotation` (`self.Propeller1`) (struct :`Yaw` -3500.0) false false)
  (`SceneComponent.K2_AddRelativeRotation` (`self.Propeller3`) (struct :`Yaw` -3500.0) false false))

(event `InputAxis|Right Thumbstrick Y`
  (params (AxisValue :type "Float (single-precision)"))
  (bind _returnvalue (`GameplayStatics.GetWorldDeltaSeconds`))
  ;[1 1 1] XYMove
  (`|ExecutionSequence`
    (:`then_0`
      (if (> AxisValue 0.0)
        (bind (_direction _newtrack_0) (`Timeline|Timeline` :!label _label_3)
          (:`Update`
            (bind _output_get (set `self.Speed` _newtrack_0))
            (`self.AddMovementInput` (`KismetMathLibrary.MakeVector` (`KismetMathLibrary.FInterpTo` 0.0 (* _output_get -1.0) _returnvalue 1.0)))))
        (else
          (goto _label_3 :!via `Reverse`))))
    (:`then_1`
      (if (< AxisValue 0.0)
        (bind (_direction_2 _newtrack_0_2) (`Timeline|Timeline_0` :!label _label_4)
          (:`Update`
            (bind _output_get_2 (set `self.Speed` _newtrack_0_2))
            (`self.AddMovementInput` (`KismetMathLibrary.MakeVector` (`KismetMathLibrary.FInterpTo` 0.0 (* _output_get_2 -1.0) _returnvalue 1.0)))))
        (else
          (goto _label_4 :!via `Reverse`))))))

(event `self.ReceiveTick`
  (params (DeltaSeconds :type "Float (single-precision)"))
  (bind _returnvalue_location (`KismetMathLibrary.BreakTransform` (`self.GetTransform`)))
  ;[1 1 1] HeightDetermination
  (bind _outhit (`KismetSystemLibrary.LineTraceSingle` _returnvalue_location (+ _returnvalue_location (* (* (`self.GetActorUpVector`) 50000.0) -1.0)) "TraceTypeQuery1"))
  (set `self.Height` (`.Distance` (`GameplayStatics.BreakHitResult` _outhit))))

(event `InputAxis|Left Thumbstrick X`
  (params (AxisValue :type "Float (single-precision)"))
  ;[1 1 1] ZRotation
  (`self.K2_AddActorLocalRotation` (`KismetMathLibrary.MakeRotator` 0.0 0.0 (* (`self.YawSpeed`) AxisValue))))

(event `InputAxis|Left Thumbstrick Y`
  (params (AxisValue :type "Float (single-precision)"))
  ;[1 1 1] Zlifting
  (if (< (`self.GetInputAxisValue`) 0.0)
    (if (<= (`self.Height`) 50.0)
      (set `self.ZSpeed` 50.0)
      (`self.AddMovementInput` (`KismetMathLibrary.MakeVector` 0.0 0.0 (`KismetMathLibrary.FInterpTo` 0.0 (* (`self.ZSpeed`) (`self.GetInputAxisValue`)) (`GameplayStatics.GetWorldDeltaSeconds`) 1.0)))
      (elif (<= (`self.Height`) 250.0)
        (set `self.ZSpeed` 100.0)
        (`self.AddMovementInput` (`KismetMathLibrary.MakeVector` 0.0 0.0 (`KismetMathLibrary.FInterpTo` 0.0 (* (`self.ZSpeed`) (`self.GetInputAxisValue`)) (`GameplayStatics.GetWorldDeltaSeconds`) 1.0)))
        (else
          (set `self.ZSpeed` 300.0)
          (`self.AddMovementInput` (`KismetMathLibrary.MakeVector` 0.0 0.0 (`KismetMathLibrary.FInterpTo` 0.0 (* (`self.ZSpeed`) (`self.GetInputAxisValue`)) (`GameplayStatics.GetWorldDeltaSeconds`) 1.0))))))
    (else
      (set `self.ZSpeed` 500.0)
      (`self.AddMovementInput` (`KismetMathLibrary.MakeVector` 0.0 0.0 (`KismetMathLibrary.FInterpTo` 0.0 (* (`self.ZSpeed`) AxisValue) (`GameplayStatics.GetWorldDeltaSeconds`) 1.0))))))

(event `Body RotationTick`
  (bind (_relativerotation_roll _relativerotation_pitch) (`KismetMathLibrary.BreakRotator` (`SceneComponent.RelativeRotation` (`self.Drone`))))
  ;[1 1 1] BodyRotation
  (`SceneComponent.K2_SetRelativeRotation` (`self.Drone`) (`KismetMathLibrary.MakeRotator` (`KismetMathLibrary.FInterpTo` _relativerotation_roll (`KismetMathLibrary.Lerp` 0.0 35.0 (`self.GetInputAxisValue`)) (`GameplayStatics.GetWorldDeltaSeconds`) 4.0) (`KismetMathLibrary.FInterpTo` _relativerotation_pitch (`KismetMathLibrary.Lerp` 0.0 35.0 (`self.GetInputAxisValue`)) (`GameplayStatics.GetWorldDeltaSeconds`) 4.0)) false false))

(fn `UserConstructionScript`)