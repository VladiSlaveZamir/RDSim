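; Prototype pawn for a player-flown drone, steered by gamepad thumbsticks.
; Sticks drive yaw and planar movement, while looping timers handle eased body tilt and counter-rotating propeller spin.
; Left-stick Y runs a downward ground trace, though every branch applies the same upward input.
; The first collision enables physics on the box, disables input and, after a delay, opens SecondLevel_Gameplay.
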(event `self.ReceiveBeginPlay`
  ;[1 1 1] RotationsTicks
  (`KismetSystemLibrary.K2_SetTimerDelegate` (`|CreateDelegate` :!event `Body RotationTick`) 0.01 true)
  (`KismetSystemLibrary.K2_SetTimerDelegate` (`|CreateDelegate` :!event `Propeller Rotation Tick`) 0.01 true))

(event `InputAxis|Left Thumbstrick X`
  (params (AxisValue :type "Float (single-precision)"))
  ;[1 1 1] Z Rotation
  (`self.K2_AddActorLocalRotation` (`KismetMathLibrary.MakeRotator` 0.0 0.0 (* (`self.YawSpeed`) AxisValue))))

(event `InputAxis|Right Thumbstrick Y`
  (params (AxisValue :type "Float (single-precision)"))
  ;[0.9263 0.99 1] Body Movement XY Plane
  (`self.AddMovementInput` (`SceneComponent.GetForwardVector` (`self.Box`)) (* (* (`self.Speed`) (`self.GetInputAxisValue`)) -1.0)))

(event `Body RotationTick`
  (bind (_relativerotation_roll _relativerotation_pitch) (`KismetMathLibrary.BreakRotator` (`SceneComponent.RelativeRotation` (`self.DroneMesh`))))
  ;[1 1 1] Body Rotation XY Plane
  (`SceneComponent.K2_SetRelativeRotation` (`self.DroneMesh`) (`KismetMathLibrary.MakeRotator` (`KismetMathLibrary.FInterpTo` _relativerotation_roll (`KismetMathLibrary.Lerp` 0.0 35.0 (`self.GetInputAxisValue`)) (`GameplayStatics.GetWorldDeltaSeconds`) 4.0) (`KismetMathLibrary.FInterpTo` _relativerotation_pitch (`KismetMathLibrary.Lerp` 0.0 35.0 (`self.GetInputAxisValue`)) (`GameplayStatics.GetWorldDeltaSeconds`) 4.0)) false false))

(event `InputAxis|Right Thumbstrick X`
  (params (AxisValue :type "Float (single-precision)"))
  ;[0.9263 0.99 1] Body Movement XY Plane
  (`self.AddMovementInput` (`SceneComponent.GetRightVector` (`self.Box`)) (* (`self.GetInputAxisValue`) (`self.Speed`))))

(event `Propeller Rotation Tick`
  ;[1 1 1] Comment
  (`SceneComponent.K2_AddRelativeRotation` (`self.Propeller2`) (struct :`Yaw` 3500.0) false false)
  (`SceneComponent.K2_AddRelativeRotation` (`self.Propeller`) (struct :`Yaw` 3500.0) false false)
  (`SceneComponent.K2_AddRelativeRotation` (`self.Propeller3`) (struct :`Yaw` -3500.0) false false)
  (`SceneComponent.K2_AddRelativeRotation` (`self.Propeller1`) (struct :`Yaw` -3500.0) false false))

(event `self.Box.OnComponentHit`
  (params (HitComponent :type "PrimitiveComponent Object Reference") (OtherActor :type "Actor Object Reference") (OtherComp :type "PrimitiveComponent Object Reference") (NormalImpulse :type "Vector Structure") (Hit :type "HitResult Structure (by ref)"))
  ;[1 1 1] Comment
  (`/Engine/EditorBlueprintResources/StandardMacros.DoOnce` false
    (:`Completed`
      (`KismetSystemLibrary.PrintString` (`KismetSystemLibrary.GetDisplayName` OtherActor))
      (`PrimitiveComponent.SetSimulatePhysics` (`self.Box`) true)
      (`self.DisableInput` (`GameplayStatics.GetPlayerController` 0))
      (`KismetSystemLibrary.Delay` 2.0)
      (`GameplayStatics.OpenLevel` "SecondLevel_Gameplay"))))

(event `InputAxis|Left Thumbstrick Y`
  (params (AxisValue :type "Float (single-precision)"))
  (bind _returnvalue_location (`KismetMathLibrary.BreakTransform` (`self.GetTransform`)))
  ;[1 1 1] LineTrace
  (bind _outhit (`KismetSystemLibrary.LineTraceSingle` :`Start` _returnvalue_location :`End` (+ _returnvalue_location (* (* (`self.GetActorUpVector`) 250.0) -1.0)) :`TraceChannel` "TraceTypeQuery1" :`DrawDebugType` "ForOneFrame"))
  (if (< (`self.GetInputAxisValue`) 0.0)
    (bind (_bblockinghit _binitialoverlap _time _distance) (`GameplayStatics.BreakHitResult` _outhit))
    (if (<= _distance 50.0)
      (`self.AddMovementInput` (`SceneComponent.GetUpVector` (`self.Box`)))
      (elif (or (<= _distance 250.0) (not (== _distance 0.0)))
        (`self.AddMovementInput` (`SceneComponent.GetUpVector` (`self.Box`)))
        (else
          (`self.AddMovementInput` (`SceneComponent.GetUpVector` (`self.Box`))))))
    (else
      (`self.AddMovementInput` (`SceneComponent.GetUpVector` (`self.Box`))))))

(fn `UserConstructionScript`)