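; Prototype player-flown drone: the left stick controls climb and yaw, the right stick horizontal movement.
; Tick reshapes right-stick input by quadrant, projecting off-axis input onto diagonals, rescaling and clamping it.
; The result drives movement and BodyRotationTick, which eases the drone mesh's pitch and roll toward a tilt.
; The first box hit prints the other actor, enables physics and disables input, so the drone crashes.
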(event `self.ReceiveBeginPlay`
  (`KismetSystemLibrary.K2_SetTimerDelegate` (`|CreateDelegate` :!event `Body RotationTick`) 0.01 true))

(event `Body RotationTick`
  (bind (_rightjoystick2daxises_x _rightjoystick2daxises_y) (`KismetMathLibrary.BreakVector2D` (`self.RightJoystick2dAxises`)))
  (bind (_relativerotation_roll _relativerotation_pitch) (`KismetMathLibrary.BreakRotator` (`SceneComponent.RelativeRotation` (`self.Drone`))))
  (`SceneComponent.K2_SetRelativeRotation` (`self.Drone`) (`KismetMathLibrary.MakeRotator` (`KismetMathLibrary.FInterpTo` _relativerotation_roll (`KismetMathLibrary.Lerp` 0.0 35.0 _rightjoystick2daxises_x) (`GameplayStatics.GetWorldDeltaSeconds`) 4.0) (`KismetMathLibrary.FInterpTo` _relativerotation_pitch (`KismetMathLibrary.Lerp` 0.0 35.0 _rightjoystick2daxises_y) (`GameplayStatics.GetWorldDeltaSeconds`) 4.0)) false false))

(event `InputAxis|Right Thumbstrick Y`
  (params (AxisValue :type "Float (single-precision)"))
  (bind (_rightjoystick2daxises_x _rightjoystick2daxises_y) (`KismetMathLibrary.BreakVector2D` (`self.RightJoystick2dAxises`)))
  (`self.AddMovementInput` (`SceneComponent.GetForwardVector` (`self.Box`)) (* (* (`self.Speed`) _rightjoystick2daxises_y) -1.0)))

(event `InputAxis|Right Thumbstrick X`
  (params (AxisValue :type "Float (single-precision)"))
  (bind _rightjoystick2daxises_x (`KismetMathLibrary.BreakVector2D` (`self.RightJoystick2dAxises`)))
  (`self.AddMovementInput` (`SceneComponent.GetRightVector` (`self.Box`)) (* _rightjoystick2daxises_x (`self.Speed`))))

(event `InputAxis|Left Thumbstrick Y`
  (params (AxisValue :type "Float (single-precision)"))
  ;[1 1 1] Подъем дрона
  (`self.AddMovementInput` (`SceneComponent.GetUpVector` (`self.Box`)) (* AxisValue (`self.Speed`))))

(event `InputAxis|Left Thumbstrick X`
  (params (AxisValue :type "Float (single-precision)"))
  ;[1 1 1] Поворот дрона
  (`self.K2_AddActorLocalRotation` (`KismetMathLibrary.MakeRotator` 0.0 0.0 (* (`self.YawSpeed`) AxisValue))))

(event `self.ReceiveTick`
  (params (DeltaSeconds :type "Float (single-precision)"))
  (bind _returnvalue (`self.GetInputAxisValue`))
  (bind _returnvalue_2 (`self.GetInputAxisValue`))
  (bind _leftxypolarangle (`self.LeftXYPolarAngle`))
  (bind _leftxypolarangle_2 (`self.LeftXYPolarAngle`))
  (bind _leftxypolarangle_3 (`self.LeftXYPolarAngle`))
  (bind _leftxypolarangle_4 (`self.LeftXYPolarAngle`))
  (bind (_returnvalue_roll _returnvalue_pitch _returnvalue_yaw) (`KismetMathLibrary.BreakRotator` (`KismetMathLibrary.FindLookAtRotation` (`SceneComponent.RelativeLocation` (`self.Drone`)) (`KismetMathLibrary.MakeVector` (`self.GetInputAxisValue`) (`self.GetInputAxisValue`)))))
  (bind _returnvalue_3 (+ _returnvalue_yaw 180.0))
  (bind (_returnvalue_x _returnvalue_y) (`KismetMathLibrary.BreakVector` (/ (`KismetMathLibrary.ProjectVectorOnToVector` (`KismetMathLibrary.MakeVector` (`self.GetInputAxisValue`) (`self.GetInputAxisValue`)) (`KismetMathLibrary.MakeVector` 1.0 1.0)) (0.6 0.6 0.6))))
  (bind (_returnvalue_x_2 _returnvalue_y_2) (`KismetMathLibrary.BreakVector` (/ (`KismetMathLibrary.ProjectVectorOnToVector` (`KismetMathLibrary.MakeVector` (`self.GetInputAxisValue`) (`self.GetInputAxisValue`)) (`KismetMathLibrary.MakeVector` -1.0 1.0)) (0.6 0.6 0.6))))
  (bind (_returnvalue_x_3 _returnvalue_y_3) (`KismetMathLibrary.BreakVector` (/ (`KismetMathLibrary.ProjectVectorOnToVector` (`KismetMathLibrary.MakeVector` (`self.GetInputAxisValue`) (`self.GetInputAxisValue`)) (`KismetMathLibrary.MakeVector` -1.0 1.0)) (0.6 0.6 0.6))))
  (bind _returnvalue_4 (`KismetMathLibrary.Abs` _returnvalue_x))
  (bind _returnvalue_5 (`KismetMathLibrary.Abs` _returnvalue_x_2))
  (bind _returnvalue_6 (`KismetMathLibrary.Abs` _returnvalue_x_3))
  (bind _returnvalue_7 (/ _returnvalue_x _returnvalue_4))
  (if (not (and (== (`self.GetInputAxisValue`) 0.0) (== (`self.GetInputAxisValue`) 0.0)))
    (set `self.E_MoveState` "NewEnumerator1")
    (set `self.LeftXYPolarAngle` _returnvalue_3)
    (if (== (mod _returnvalue_3 90.0) 0.0)
      (switch `int` (`KismetMathLibrary.FTrunc` (/ _returnvalue_3 90.0))
        (:`1`
          (set `self.RightJoystick2dAxises` (`KismetMathLibrary.MakeVector2D` 0.0 _returnvalue_2)))
        (:`2`
          (set `self.RightJoystick2dAxises` (`KismetMathLibrary.MakeVector2D` _returnvalue)))
        (:`3`
          (set `self.RightJoystick2dAxises` (`KismetMathLibrary.MakeVector2D` 0.0 _returnvalue_2)))
        (:`4`
          (set `self.RightJoystick2dAxises` (`KismetMathLibrary.MakeVector2D` _returnvalue))))
      (elif (or (and (> _leftxypolarangle_2 0.0) (< _leftxypolarangle_2 90.0)) (and (> _leftxypolarangle_4 180.0) (< _leftxypolarangle_4 270.0)))
        (if (> _returnvalue_4 1.0)
          (set `self.RightJoystick2dAxises` (`KismetMathLibrary.MakeVector2D` _returnvalue_7 _returnvalue_7))
          (else
            (set `self.RightJoystick2dAxises` (`KismetMathLibrary.MakeVector2D` _returnvalue_x _returnvalue_y))))
        (elif (and (> _leftxypolarangle_3 90.0) (< _leftxypolarangle_3 180.0))
          (if (> _returnvalue_6 1.0)
            (set `self.RightJoystick2dAxises` (`KismetMathLibrary.MakeVector2D` (/ _returnvalue_x_3 _returnvalue_6) (/ (`KismetMathLibrary.Abs` _returnvalue_y_3) _returnvalue_y_3)))
            (else
              (set `self.RightJoystick2dAxises` (`KismetMathLibrary.MakeVector2D` _returnvalue_x_3 _returnvalue_y_3))))
          (elif (and (> _leftxypolarangle 270.0) (< _leftxypolarangle 360.0))
            (if (> _returnvalue_5 1.0)
              (set `self.RightJoystick2dAxises` (`KismetMathLibrary.MakeVector2D` (/ _returnvalue_x_2 _returnvalue_5) (/ (`KismetMathLibrary.Abs` _returnvalue_y_2) _returnvalue_y_2)))
              (else
                (set `self.RightJoystick2dAxises` (`KismetMathLibrary.MakeVector2D` _returnvalue_x_2 _returnvalue_y_2))))))))
    (else
      (set `self.RightJoystick2dAxises` (0.0 0.0))
      (set `self.E_MoveState` "NewEnumerator0"))))

(event `self.Box.OnComponentHit`
  (params (HitComponent :type "PrimitiveComponent Object Reference") (OtherActor :type "Actor Object Reference") (OtherComp :type "PrimitiveComponent Object Reference") (NormalImpulse :type "Vector Structure") (Hit :type "HitResult Structure (by ref)"))
  (`/Engine/EditorBlueprintResources/StandardMacros.DoOnce` false
    (:`Completed`
      (`KismetSystemLibrary.PrintString` (`KismetSystemLibrary.GetDisplayName` OtherActor))
      (`PrimitiveComponent.SetSimulatePhysics` (`self.Box`) true)
      (`self.DisableInput` (`GameplayStatics.GetPlayerController` 0))
      (`KismetSystemLibrary.Delay` 2.0))))

(fn `UserConstructionScript`)